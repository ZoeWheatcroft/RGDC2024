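; Start elevator Blueprint with a door that opens and closes as the player passes its triggers.
; Box overlap by BP_PlayerCharacter calls OpenDoor, while CloseTrigger overlap by player pawn 0 calls CloseDoor.
; Each plays its own timeline from the start to set the Door's relative rotation.
; The timeline value becomes a Y-only direction vector converted to a rotator, so only its sign affects the resulting yaw.
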(event `self.ReceiveBeginPlay`
  (add `PrimitiveComponent.OnComponentBeginOverlap` (`self.Box`) (delegate `CustomEvent`)))

(event `CustomEvent`
  (params (OverlappedComponent :type "PrimitiveComponent Object Reference") (OtherActor :type "Actor Object Reference") (OtherComp :type "PrimitiveComponent Object Reference") (OtherBodyIndex :type Integer) (bFromSweep :type Boolean) (SweepResult :type "HitResult Structure (by ref)"))
  (cast `/Game/PBController/BP_PlayerCharacter` OtherActor)
  (`self.Open Door`))

(event `Open Door`
  (bind (_direction _doorrotation) (`Timeline|Timeline` :!via `PlayFromStart`)
    (:`Update`
      (`SceneComponent.K2_SetRelativeRotation` (`self.door`) (`KismetMathLibrary.Conv_VectorToRotator` (`KismetMathLibrary.MakeVector` 0.0 _doorrotation)) false false))))

(event `self.close trigger.OnComponentBeginOverlap`
  (params (OverlappedComponent :type "PrimitiveComponent Object Reference") (OtherActor :type "Actor Object Reference") (OtherComp :type "PrimitiveComponent Object Reference") (OtherBodyIndex :type Integer) (bFromSweep :type Boolean) (SweepResult :type "HitResult Structure (by ref)"))
  (if (== OtherActor (`GameplayStatics.GetPlayerCharacter` 0))
    (`self.CloseDoor`)))

(event `CloseDoor`
  (bind (_direction _newtrack_1) (`Timeline|Timeline_0` :!via `PlayFromStart`)
    (:`Update`
      (`SceneComponent.K2_SetRelativeRotation` (`self.door`) (`KismetMathLibrary.Conv_VectorToRotator` (`KismetMathLibrary.MakeVector` 0.0 _newtrack_1)) false false))))

(fn `UserConstructionScript`)