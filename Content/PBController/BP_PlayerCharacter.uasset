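; Player character Blueprint with noclip toggling, a health component, a gun component and an on-screen HUD.
; BeginPlay creates the WP_Hud widget and adds it to the viewport.
; The Health component's OnHit event writes current health minus the incoming damage to the HUD's health text.
; GetAmmo exposes the gun component's ammo, and TESTUI deals fixed test damage through the Health component.
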(event `InputAction|ToggleNoclip`
  (params (Key :type "Key Structure"))
  (:`Pressed`
    (`self.ToggleNoClip`)))

(event `self.ReceiveBeginPlay`
  (bind _returnvalue (`|CreateWidget` "/Game/Hud/WP_Hud.WP_Hud_C"))
  (bind _output_get (set `self.HudRef` _returnvalue))
  (`UserWidget.AddToViewport` _output_get 0))

(event `self.Health.OnHit`
  (params (DamageTaken :type "Float (single-precision)"))
  (`TextBlock.SetText` (`/Game/Hud/WP_HealthText.HealthDisplay` (`/Game/Hud/WP_Hud.WP_HealthText` (`self.HudRef`))) (`KismetTextLibrary.Conv_DoubleToText` (- (`HealthComponent.GetHealth` (`self.Health`)) DamageTaken) "HalfToEven")))

(fn `GetAmmo`
  (returns (NewParam :type Integer))
  (return (`/Game/Chargul/BP_GunComponent.Ammo` (`self.BP_GunComponent`))))

(fn `TESTUI`
  (`HealthComponent.Damage` (`self.Health`) 3.0))

(fn `UserConstructionScript`)