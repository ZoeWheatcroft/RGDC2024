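; BP_BaseWeapon is a base weapon Blueprint with a hitscan fire test and a simple ammo reload.
; Left mouse runs a persistently drawn Visibility line trace forward from the camera and destroys any StaticMeshActor it hits.
; Tick watches Ammo and calls Reload after a delay once it is empty, restoring the starting count.
; Firing never consumes Ammo, and the Shoot function is an empty stub.
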(event `self.ReceiveBeginPlay`
  (set `self.Ammo` 6))

(event `self.ReceiveTick`
  (params (DeltaSeconds :type "Float (single-precision)"))
  (if (<= (`self.Ammo`) 0)
    (`KismetSystemLibrary.Delay` 3.0)
    (`self.Reload`)))

(event `Key|LeftMouseButton`
  (params (Key :type "Key Structure"))
  (bind _camera (`self.Camera`))
  (bind _returnvalue (`SceneComponent.K2_GetComponentLocation` _camera))
  (:`Pressed`
    (bind _outhit (`KismetSystemLibrary.LineTraceSingle` :`Start` _returnvalue :`End` (+ _returnvalue (* (`SceneComponent.GetForwardVector` _camera) (`self.TraceLength`))) :`TraceChannel` "TraceTypeQuery1" :`DrawDebugType` "Persistent"))
    (bind _asstatic_mesh_actor (cast `StaticMeshActor` (`.HitActor` (`GameplayStatics.BreakHitResult` _outhit))))
    (`self.K2_DestroyActor` _asstatic_mesh_actor)))

(fn `Reload`
  (set `self.Ammo` 6))

(fn `Shoot`)

(fn `UserConstructionScript`)