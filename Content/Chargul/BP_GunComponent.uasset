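; Gun component that fires a hitscan laser on left mouse click, destroying any static mesh actor it hits.
; A visibility line trace runs from the player camera, and a Niagara beam spawns just below it, ending at full trace length regardless of hits.
; Tick triggers a delayed reload to max ammo when ammo is empty, but firing neither checks nor consumes ammo.
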(event `self.ReceiveTick`
  (params (DeltaSeconds :type "Float (single-precision)"))
  (if (<= (`self.Ammo`) 0)
    (`KismetSystemLibrary.Delay` 3.0)
    (`self.Reload`)))

(event `self.ReceiveBeginPlay`
  (set `self.Ammo` 1)
  (set `self.PlayerCameraVar` (`Actor.GetComponentByClass` (`self.GetOwner`) "/Script/Engine.CameraComponent")))

(event `Key|LeftMouseButton`
  (params (Key :type "Key Structure"))
  (bind _returnvalue (`GameplayStatics.GetPlayerCameraManager` 0))
  (bind _returnvalue_2 (`PlayerCameraManager.GetCameraLocation` _returnvalue))
  (bind _returnvalue_3 (+ _returnvalue_2 (* (`KismetMathLibrary.GetForwardVector` (`PlayerCameraManager.GetCameraRotation` _returnvalue)) (`self.TraceLength`))))
  (:`Pressed`
    (bind _outhit (`KismetSystemLibrary.LineTraceSingle` _returnvalue_2 _returnvalue_3 "TraceTypeQuery1" false (`|MakeArray` (`self.GetOwner`))))
    (bind _returnvalue_4 (`NiagaraFunctionLibrary.SpawnSystemAtLocation` "/Game/Chargul/NS_Laser.NS_Laser" (- _returnvalue_2 (0.0 0.0 50.0)) (struct) (1.0 1.0 1.0) false))
    (`NiagaraComponent.SetVariableVec3` _returnvalue_4 "Beam End" _returnvalue_3)
    (bind _asstatic_mesh_actor (cast `StaticMeshActor` (`.HitActor` (`GameplayStatics.BreakHitResult` _outhit))))
    (`Actor.K2_DestroyActor` _asstatic_mesh_actor)))

(fn `Reload`
  (set `self.Ammo` (`self.MaxAmmo`)))