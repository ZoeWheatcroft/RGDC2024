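; BP_Ostrich is a ranged enemy that shoots at a target and explodes on death.
; Its Attack function spawns a BP_OstrichProjectile at the spawn point and passes it the target to shoot at.
; The Health component's OnDied event triggers SelfDestruct, which plays a Niagara explosion, fires a radial impulse, damages the player if inside the hurt zone, then destroys the actor.
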(event `self.Health.OnDied`
  (`self.SelfDestruct`))

(fn `Attack`
  (params (Target :type "Vector Structure (by ref)"))
  (locals (Player :type "Vector Structure"))
  (set `local.Player` Target)
  (bind _returnvalue (`|SpawnActorFromClass` "/Game/AI/Ostrich/BP_OstrichProjectile.BP_OstrichProjectile_C" (`KismetMathLibrary.Conv_VectorToTransform` (`SceneComponent.K2_GetComponentLocation` (`self.ProjectileSpawnPoint`))) "Undefined" "MultiplyWithRoot" null self))
  (`/Game/AI/Ostrich/BP_OstrichProjectile.ShootProjectile` _returnvalue (`local.Player`)))

(fn `SelfDestruct`
  (`NiagaraFunctionLibrary.SpawnSystemAtLocation` "/Game/MixedVFX/Particles/Explosions/NS_ExplosionGroundSmall.NS_ExplosionGroundSmall" (`self.K2_GetActorLocation`))
  (`RadialForceComponent.FireImpulse` (`self.RadialForce`))
  (if (`PrimitiveComponent.IsOverlappingActor` (`self.SelfDestructHurtZone`) (`GameplayStatics.GetPlayerPawn` 0))
    (`GameplayStatics.ApplyDamage` (`GameplayStatics.GetPlayerPawn` 0) 2.0))
  (`self.K2_DestroyActor`))

(fn `UserConstructionScript`
  (`parent.UserConstructionScript`))